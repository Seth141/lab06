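; Player character with mouse-look that uses a gaze check to interact with objects or teleport.
; Every tick, a debug-drawn Visibility line trace from the camera stores any hit actor implementing the Interaction interface as InteractingActor.
; Left click sends InteractMessage to that actor, or otherwise teleports to the trace's hit location without checking for a hit.
; Old cube-detection and forward-movement nodes are disconnected, and the Interact function is empty.
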(event `InputAction|leftClick`
  (params (Key :type "Key Structure"))
  (bind _interactingactor (`self.interactingActor`))
  (:`Pressed`
    (`/Engine/EditorBlueprintResources/StandardMacros.IsValid` _interactingactor
      (:`Is Valid`
        (`|ExecutionSequence`
          (:`then_1`
            (message `/Game/Blueprints/Interaction.Interact` _interactingactor))))
      (:`Is Not Valid`
        (if (not (`KismetSystemLibrary.DoesImplementInterface` _interactingactor "/Game/Blueprints/Interaction.Interaction_C"))
          (`self.K2_TeleportTo` (`.Location` (`GameplayStatics.BreakHitResult` (stale `GazeCheck` _outhit)))))))))

(event `self.ReceiveTick`
  (params (DeltaSeconds :type "Float (single-precision)"))
  (`self.GazeCheck`))

(event `InputAxis|mouseX`
  (params (AxisValue :type "Float (single-precision)"))
  ;[1 1 1] Input
  (`self.AddControllerYawInput` AxisValue))

(event `InputAxis|mouseY`
  (params (AxisValue :type "Float (single-precision)"))
  ;[1 1 1] Input
  (`self.AddControllerPitchInput` AxisValue))

(event `GazeCheck`
  (bind _camera (`self.Camera`))
  (bind _returnvalue (`SceneComponent.K2_GetComponentLocation` _camera))
  ;[1 1 1] Gaze check
  (bind _outhit (`KismetSystemLibrary.LineTraceSingle` :`Start` _returnvalue :`End` (+ _returnvalue (* (`SceneComponent.GetForwardVector` _camera) 2000)) :`TraceChannel` "TraceTypeQuery1" :`DrawDebugType` "ForOneFrame"))
  (bind (_bblockinghit _binitialoverlap _time _distance _location _impactpoint _normal _impactnormal _physmat _hitactor) (`GameplayStatics.BreakHitResult` _outhit))
  (if (`KismetSystemLibrary.DoesImplementInterface` _hitactor "/Game/Blueprints/Interaction.Interaction_C")
    (set `self.interactingActor` _hitactor)
    (else
      (set `self.interactingActor` null))))

(fn `Interact`)

(fn `UserConstructionScript`)