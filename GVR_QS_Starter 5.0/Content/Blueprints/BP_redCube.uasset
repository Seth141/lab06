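; Interactable red cube actor that, once triggered, fades the material opacity of its Boo component according to whether the actor is on screen.
; Interact prints a taunt, clears the cube mesh and the OminousWarning text, then sets the Begin flag.
; While Begin is set, Tick uses WasRecentlyRendered to play or reverse a timeline that drives Boo's Opacity parameter.
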(event `self.ReceiveBeginPlay`)

(event `self.ReceiveTick`
  (params (DeltaSeconds :type "Float (single-precision)"))
  (if (`self.begin`)
    (if (`self.WasRecentlyRendered` 0.2)
      (bind (_direction _changeopacity) (`Timeline|Timeline_0` :!label _label)
        (:`Update`
          (`MeshComponent.SetScalarParameterValueOnMaterials` (`self.boo`) "Opacity" _changeopacity)))
      (else
        (goto _label :!via `Reverse`)))))

(event `/Game/Blueprints/Interaction.Interact`
  (`|ExecutionSequence`
    (:`then_0`
      (`KismetSystemLibrary.PrintString` "YOU FOOL")
      (`StaticMeshComponent.SetStaticMesh` (`self.Cube`) null)
      (`TextRenderComponent.K2_SetText` (`self.ominousWarning`) (`KismetTextLibrary.GetEmptyText`)))
    (:`then_1`
      (set `self.begin` true))))

(fn `UserConstructionScript`)